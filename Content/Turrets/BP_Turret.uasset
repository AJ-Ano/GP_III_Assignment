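; Turret actor that turns its static mesh to face a player-tagged actor inside its detection component.
; Overlap begin stores the target and starts a looping half-second timer, and overlap end clears that timer while keeping the target reference.
; Each timer tick interpolates the mesh's relative yaw toward the look-at rotation from the turret to the target, leaving pitch and roll at zero.
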(event `self.Player Detection.OnComponentBeginOverlap`
  (params (OverlappedComponent :type "PrimitiveComponent Object Reference") (OtherActor :type "Actor Object Reference") (OtherComp :type "PrimitiveComponent Object Reference") (OtherBodyIndex :type Integer) (bFromSweep :type Boolean) (SweepResult :type "HitResult Structure (by ref)"))
  ; See Player Start Tracking
  (`/Engine/EditorBlueprintResources/StandardMacros.IsValid` OtherActor
    (:`Is Valid`
      (if (`self.ActorHasTag` OtherActor "player")
        (set `self.Target` OtherActor)
        (`self.TrackTarget`)))))

(event `self.Player Detection.OnComponentEndOverlap`
  (params (OverlappedComponent :type "PrimitiveComponent Object Reference") (OtherActor :type "Actor Object Reference") (OtherComp :type "PrimitiveComponent Object Reference") (OtherBodyIndex :type Integer))
  ; When Player Leave Turret Range Stop Tracking
  (`/Engine/EditorBlueprintResources/StandardMacros.IsValid` OtherActor
    (:`Is Valid`
      (if (`self.ActorHasTag` OtherActor "player")
        (`self.Target`
          (:`then`
            (`KismetSystemLibrary.K2_ClearAndInvalidateTimerHandle` (`self.TimerRef`)))
          (:`else`))))))

(event `TrackTarget`
  ; Rotating Turret
  (bind _returnvalue (`KismetSystemLibrary.K2_SetTimerDelegate` (delegate `MoveTurret`) 0.5 true true))
  (set `self.TimerRef` _returnvalue))

(event `MoveTurret`
  (bind _target (`self.Target`))
  (bind (_returnvalue_roll _returnvalue_pitch _returnvalue_yaw) (`KismetMathLibrary.BreakRotator` (`KismetMathLibrary.RInterpTo` (`SceneComponent.RelativeRotation` (`self.StaticMesh`)) (`KismetMathLibrary.FindLookAtRotation` (`self.K2_GetActorLocation`) (`self.K2_GetActorLocation` _target)) (`GameplayStatics.GetWorldDeltaSeconds`) 100.0)))
  ; Rotating Turret
  (`/Engine/EditorBlueprintResources/StandardMacros.IsValid` _target
    (:`Is Valid`
      (`SceneComponent.K2_SetRelativeRotation` (`self.StaticMesh`) (`KismetMathLibrary.MakeRotator` 0.0 0.0 _returnvalue_yaw) false false))))

(fn `UserConstructionScript`)