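; BP_MyGameMode is a game mode Blueprint that runs an on-screen countdown from the start of play.
; BeginPlay creates the WB_CountdownTimer widget, adds it to the viewport and starts a looping one-second timer.
; Each TakeCountdown tick decrements Count, writes it to the widget's text and clears the timer at zero, with no further action on expiry.
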(event `Take Countdown`
  (`/Engine/EditorBlueprintResources/StandardMacros.DecrementInt` (`self.Count`)
    (:`  `
      (`TextBlock.SetText` (`/Game/HUD/WB_CountdownTimer.CountdownText` (`self.CountdownWidget`)) (`KismetTextLibrary.Conv_IntToText` (`self.Count`)))
      (if (<= (`self.Count`) 0)
        (`KismetSystemLibrary.K2_ClearAndInvalidateTimerHandle` (stale `self.ReceiveBeginPlay` _returnvalue_2))))))

(event `self.ReceiveBeginPlay`
  (bind _returnvalue (`|CreateWidget` "/Game/HUD/WB_CountdownTimer.WB_CountdownTimer_C"))
  (bind _output_get (set `self.CountdownWidget` _returnvalue))
  (`UserWidget.AddToViewport` _output_get 0)
  (bind _returnvalue_2 (`KismetSystemLibrary.K2_SetTimerDelegate` (delegate `Take Countdown`) 1.0 true)))

(fn `UserConstructionScript`)